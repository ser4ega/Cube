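; Player pawn for BananaCollector that moves along forward, right and up input axes.
; Axis input is scaled by Maxspeed along actor vectors, then consumed each Tick as a swept, delta-time-scaled local offset, though the vectors are in world space.
; Jumping is unfinished: press and release only set the Jumpstart and Jumped flags to false, the Jump function is empty, and two Delay nodes are unconnected.
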(event `InputAxis|forward`
  (params (AxisValue :type "Float (single-precision)"))
  (`self.AddMovementInput` (`self.GetActorForwardVector`) (* (`self.maxspeed`) AxisValue)))

(event `InputAxis|right`
  (params (AxisValue :type "Float (single-precision)"))
  (`self.AddMovementInput` (`self.GetActorRightVector`) (* (`self.maxspeed`) AxisValue)))

(event `InputAxis|up`
  (params (AxisValue :type "Float (single-precision)"))
  (`self.AddMovementInput` (`self.GetActorUpVector`) (* (`self.maxspeed`) AxisValue)))

(event `self.ReceiveTick`
  (params (DeltaSeconds :type "Float (single-precision)"))
  (bind _returnvalue (`self.ConsumeMovementInputVector`))
  (`self.K2_AddActorLocalOffset` (* _returnvalue DeltaSeconds) true))

(event `InputAction|jump`
  (params (Key :type "Key Structure"))
  (:`Pressed`
    (set `self.jumpstart` false))
  (:`Released`
    (set `self.jumped` false)))

(fn `jump`
  (params (NewParam :type Boolean)))

(fn `UserConstructionScript`)